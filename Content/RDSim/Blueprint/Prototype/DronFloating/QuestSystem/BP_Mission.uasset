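; BP_Mission is a single mission in the quest system of the DronFloating prototype, tracking its state and numeric phase.
; Init stores the mission info and owning player pawn and resets the phase.
; UpdateState and UpdatePhase set the new value and broadcast it with the mission through event dispatchers.
; Phase changes also print an on-screen debug message, while the matching state print is disconnected.
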(fn ConstructionScript)

(fn Init
  (params (InMissionInfo :type Struct%20Mission%20Info%20Structure) (InPlayerPawn :type BP%20Drone%20Pawn%20Object%20Reference))
  (Variables|Default|SetInfo InMissionInfo)
  (Variables|Default|SetOwnerPlayerPawn InPlayerPawn)
  (Variables|Default|SetPhase 0))

(fn UpdateState
  (params (InNewState :type EMissionState%20Enum :default "EMissionState_MAX"))
  (bind _output_get (Variables|Default|SetState InNewState))
  (Default|CallOnChangedStateMission self _output_get))

(fn UpdatePhase
  (params (InNewPhase :type Integer))
  (Development|PrintString (Utilities|String|Append (Utilities|String|ToString(Text) (.nameui (Variables|Default|GetInfo))) "" "Changed phase to '" (Utilities|String|ToString(Integer) InNewPhase) "'") true true "(R=0.000000,G=0.660000,B=1.000000,A=1.000000)" 1e+01)
  (bind _output_get (Variables|Default|SetPhase InNewPhase))
  (Default|CallOnChangedPhaseMission self _output_get))