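; Mission manager for the drone prototype's quest system, holding a list of missions and tracking which one is current.
; Added missions get a waiting state, and the first becomes current if none is set; switching demotes the previous one unless finished.
; It listens only to the current mission's state changes, removing it when finished and promoting the first remaining one.
; Current-mission changes are broadcast through a dispatcher, and missions can be found by name or cleared.
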(event Custom|OnChangedStateMission
  (params (InMission :type BP%20Mission%20Object%20Reference) (InNewState :type EMissionState%20Enum :default "NewEnumerator0"))
  (bind _missions (Variables|Default|GetMissions))
  (if (Utilities|Enum|Equal(Enum) InNewState "NewEnumerator2")
    (CallFunction|RemoveMissionbyPointer InMission)
    (if (Utilities|Array|IsNotEmpty _missions)
      (CallFunction|SetCurrentMission (Utilities|Array|Get(acopy) _missions)))))

(fn ConstructionScript)

(fn AddNextMission
  (params (InMission :type BP%20Mission%20Object%20Reference))
  (Utilities|Array|Add (Variables|Default|GetMissions) InMission)
  (Default|UpdateState InMission "NewEnumerator1")
  (Utilities|IsValid (Variables|Default|GetCurrentMission)
    (:Is%20Not%20Valid
      (CallFunction|SetCurrentMission InMission))))

(fn SetCurrentMission
  (params (InMIssion :type BP%20Mission%20Object%20Reference))
  (if (!= InMIssion (Variables|Default|GetCurrentMission))
    (Utilities|IsValid (Variables|Default|GetCurrentMission)
      (:Is%20Valid
        (EventDispatchers|UnbindEventfromOnChangedStateMission (Variables|Default|GetCurrentMission) (EventDispatchers|CreateEvent :!event Custom|OnChangedStateMission))
        (if (Utilities|Enum|NotEqual(Enum) (Variables|/Game/RDSim/Blueprint/Prototype/DronFloating/QuestSystem/BP_Mission.BP_Mission_C|GetState (Variables|Default|GetCurrentMission)) "NewEnumerator2")
          (Default|UpdateState (Variables|Default|GetCurrentMission) "NewEnumerator1"))
        (Variables|Default|SetCurrentMission 0))
      (:Is%20Not%20Valid
        _))
    (Utilities|IsValid InMIssion
      (:Is%20Valid
        (bind _output_get (Variables|Default|SetCurrentMission InMIssion))
        (Default|UpdateState _output_get "NewEnumerator0")
        (EventDispatchers|BindEventtoOnChangedStateMission _output_get (EventDispatchers|CreateEvent :!event Custom|OnChangedStateMission)))
      (:Is%20Not%20Valid
        _))
    (Default|CallOnChangedCurrentMission (Variables|Default|GetCurrentMission))))

(fn RemoveAllMissions
  (CallFunction|SetCurrentMission)
  (Utilities|Array|Clear (Variables|Default|GetMissions)))

(fn RemoveMissionbyPointer
  (params (InMission :type BP%20Mission%20Object%20Reference))
  (bind _missions (Variables|Default|GetMissions))
  (Utilities|IsValid InMission
    (:Is%20Valid
      (if (== (Variables|Default|GetCurrentMission) InMission)
        (CallFunction|SetCurrentMission))
      (Utilities|Array|RemoveItem _missions InMission)
      (if (and (Utilities|Array|IsNotEmpty _missions) (not (Utilities|IsValid (Variables|Default|GetCurrentMission))))
        (CallFunction|SetCurrentMission (Utilities|Array|Get(acopy) (Variables|Default|GetMissions)))))))

(fn FindMission
  (params (InName :type Name))
  (for _array_element (Variables|Default|GetMissions)
    (if (== InName (.name (Variables|/Game/RDSim/Blueprint/Prototype/DronFloating/QuestSystem/BP_Mission.BP_Mission_C|GetInfo _array_element)))
      (return _array_element)))
  (return 0))