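; Player drone pawn flown by gamepad, with pause and level restart.
; A status state gates flight: a stick gesture arms it, traced height above 100 switches to Fly, and a chassis hit enables physics and disables it.
; Sticks drive movement, yaw and lift, with slower descent near ground; looping timers animate propellers and body tilt.
; BeginPlay queues two DataTable missions in a spawned manager, creating timers and HUD only if both rows exist.
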(event OnComponentHit(Box_Chassis)
  (params (HitComponent :type Primitive%20Component%20Object%20Reference) (OtherActor :type Actor%20Object%20Reference) (OtherComp :type Primitive%20Component%20Object%20Reference) (NormalImpulse :type Vector :default "0, 0, 0") (Hit :type Hit%20Result%20Structure%20%28by%20ref%29))
  (bind _drone (Variables|Default|GetDrone))
  ;[1 1 1] Landing
  (switch Utilities|FlowControl|Switch|SwitchonENUM_StatusDrone (Variables|Default|GetStatusDrone)
    (:NewEnumerator0
      (Physics|SetEnableGravity _drone true)
      (Physics|SetSimulatePhysics _drone true)
      (Variables|Default|SetStatusDrone "NewEnumerator3"))))

(event Custom|Propeller%20Rotation%20Tick
  ;[1 1 1] Rotation propellers
  (switch Utilities|FlowControl|Switch|SwitchonENUM_StatusDrone (Variables|Default|GetStatusDrone)
    (:NewEnumerator0
      _)
    (:NewEnumerator2
      _))
  (Transformation|AddRelativeRotation (Variables|Default|GetPropeller2) "0.000000,3500.000000,0.000000" false false)
  (Transformation|AddRelativeRotation (Variables|Default|GetPropeller1) "0.000000,-3500.000000,0.000000" false false))

(event Custom|Body%20RotationTick
  (bind _returnvalue (Utilities|Time|GetWorldDeltaSeconds))
  (bind _speeddestination (Variables|Default|GetSpeedDestination))
  (bind _drone (Variables|Default|GetDrone))
  (bind _returnvalue_2 (Math|Vector|NegateVector _speeddestination))
  (bind _relativerotation (Variables|/Script/Engine.SceneComponent|GetRelativeRotation _drone))
  ;[1 1 1] BodyRotation
  (switch Utilities|FlowControl|Switch|SwitchonENUM_StatusDrone (Variables|Default|GetStatusDrone)
    (:NewEnumerator0
      (if (not (Math|Boolean|ANDBoolean (== (Input|AxisValues|GetRightThumbstrickX) 0.0) (== (Input|AxisValues|GetRightThumbstrickY) 0.0) (!= (Math|Vector|VectorLength (Variables|Default|GetSpeedDestination)) 0.0)))
        (Transformation|SetRelativeRotation (Variables|Default|GetDrone) (Math|Rotator|MakeRotator (Math|Interpolation|FInterpTo (.roll _relativerotation) (Math|Float|Lerp 0.0 35.0 (Input|AxisValues|GetRightThumbstrickX)) (Utilities|Time|GetWorldDeltaSeconds) 1.0) (Math|Interpolation|FInterpTo (.pitch _relativerotation) (Math|Float|Lerp 0.0 35.0 (Input|AxisValues|GetRightThumbstrickY)) (Utilities|Time|GetWorldDeltaSeconds) 1.0) 0.0) false false)
        (else
          (Transformation|SetRelativeRotation (Variables|Default|GetDrone) (Math|Rotator|MakeRotator (Math|Interpolation|FInterpTo (.roll (Variables|/Script/Engine.SceneComponent|GetRelativeRotation (Variables|Default|GetDrone))) (Math|Float|Lerp 0.0 35.0 (.x _returnvalue_2)) _returnvalue 1.0) (Math|Interpolation|FInterpTo (.pitch (Variables|/Script/Engine.SceneComponent|GetRelativeRotation (Variables|Default|GetDrone))) (Math|Float|Lerp 0.0 35.0 (.y _returnvalue_2)) _returnvalue 1.0) 0.0) false false))))))

(event EventBeginPlay
  (bind _returnvalue (Game|SpawnActorfromClass "/Game/RDSim/Blueprint/Prototype/DronFloating/QuestSystem/BP_MissionManager.BP_MissionManager_C" (Transformation|GetActorTransform) "AlwaysSpawn" "MultiplyWithRoot" 0 0))
  (Variables|Default|SetMissionManager _returnvalue)
  (bind _returnvalue_2 (Utilities|GetDataTableRow "/Game/RDSim/Blueprint/Prototype/DronFloating/QuestSystem/DT_Missions.DT_Missions" "MS-1")
    (:then
      (bind _returnvalue_3 (Game|SpawnActorfromClass "/Game/RDSim/Blueprint/Prototype/DronFloating/QuestSystem/BP_Mission.BP_Mission_C" (Transformation|GetActorTransform) "AlwaysSpawn" "MultiplyWithRoot" 0 0))
      (Default|Init _returnvalue_3 _returnvalue_2 self)
      (Default|AddNextMission (Variables|Default|GetMissionManager) _returnvalue_3)
      (bind _returnvalue_4 (Utilities|GetDataTableRow "/Game/RDSim/Blueprint/Prototype/DronFloating/QuestSystem/DT_Missions.DT_Missions" "MS-2")
        (:then
          (bind _returnvalue_5 (Game|SpawnActorfromClass "/Game/RDSim/Blueprint/Prototype/DronFloating/QuestSystem/BP_Mission.BP_Mission_C" (Transformation|GetActorTransform) "AlwaysSpawn" "MultiplyWithRoot" 0 0))
          (Default|Init _returnvalue_5 _returnvalue_4 self)
          (Default|AddNextMission (Variables|Default|GetMissionManager) _returnvalue_5)
          ;[1 1 1] Propeller and Body Rotation
          (Utilities|Time|SetTimerbyEvent (EventDispatchers|CreateEvent :!event Custom|Propeller%20Rotation%20Tick) 0.01 true)
          (Utilities|Time|SetTimerbyEvent (EventDispatchers|CreateEvent :!event Custom|Body%20RotationTick) 0.01 true)
          ;[1 1 1] UI creation
          (bind _returnvalue_6 (UserInterface|CreateWidget "/Game/RDSim/Blueprint/UI/Pause_Widget.Pause_Widget_C"))
          (bind _output_get (Variables|Default|SetPause_Widjet_Reference _returnvalue_6))
          (Widget|SetVisibility _output_get "Hidden")
          (UserInterface|Viewport|AddtoViewport _output_get 0)
          (bind _returnvalue_7 (UserInterface|CreateWidget "/Game/RDSim/Blueprint/UI/BPW_DroneHUD.BPW_DroneHUD_C"))
          (UserInterface|Viewport|AddtoViewport _returnvalue_7 0)
          (Variables|Default|SetDroneHUD _returnvalue_7))))))

(event EventTick
  (params (DeltaSeconds :type Float%20%28single-precision%29))
  (bind _returnvalue (Transformation|GetActorTransform))
  (bind _returnvalue_2 (Transformation|GetVelocity))
  (bind _returnvalue_3 (Input|AxisValues|GetLeftThumbstrickY))
  (bind _returnvalue_4 (Input|AxisValues|GetRightThumbstrickX))
  ;[1 1 1] HeightDetermination
  (Variables|Default|SetVelocityLength (Math|Vector|VectorLength _returnvalue_2))
  (Variables|Default|SetSpeedDestination (/ _returnvalue_2 1805.0))
  (bind _outhit (Collision|LineTraceByChannel (.location _returnvalue) (+ (.location _returnvalue) (* (* (Transformation|GetActorUpVector) 5e+04) -1.0)) "TraceTypeQuery1" false 0 "None"))
  (Variables|Default|SetHeight (.Distance (Collision|BreakHitResult _outhit)))
  (Utilities|FlowControl|Sequence
    (:then_0
      ;[1 1 1] Landing
      (switch Utilities|FlowControl|Switch|SwitchonENUM_StatusDrone (Variables|Default|GetStatusDrone)
        (:NewEnumerator1
          (if (Math|Boolean|ANDBoolean (< _returnvalue_3 -0.7) (> _returnvalue_3 -0.9) (< _returnvalue_4 -0.7) (> _returnvalue_4 -0.9))
            (Variables|Default|SetStatusDrone "NewEnumerator2")))))
    (:then_1
      (switch Utilities|FlowControl|Switch|SwitchonENUM_StatusDrone (Variables|Default|GetStatusDrone)
        (:NewEnumerator2
          (if (> (Variables|Default|GetHeight) 1e+02)
            (Variables|Default|SetStatusDrone "NewEnumerator0")))))))

(event Input|AxisEvents|InputAxisRightThumbstrickX
  (params (AxisValue :type Float%20%28single-precision%29))
  ;[1 1 1] XYMove
  (switch Utilities|FlowControl|Switch|SwitchonENUM_StatusDrone (Variables|Default|GetStatusDrone)
    (:NewEnumerator0
      (Pawn|Input|AddMovementInput (Math|Vector|GetRightVector (Variables|Default|GetBox_Chassis)) AxisValue false))))

(event Input|AxisEvents|InputAxisLeftThumbstrickX
  (params (AxisValue :type Float%20%28single-precision%29))
  ;[1 1 1] ZRotation
  (switch Utilities|FlowControl|Switch|SwitchonENUM_StatusDrone (Variables|Default|GetStatusDrone)
    (:NewEnumerator0
      (Transformation|AddActorLocalRotation (Math|Rotator|MakeRotator 0.0 0.0 (* (Variables|Default|GetYawSpeed) AxisValue)) false false))))

(event Input|AxisEvents|InputAxisLeftThumbstrickY
  (params (AxisValue :type Float%20%28single-precision%29))
  ;[1 1 1] Zlifting
  (switch Utilities|FlowControl|Switch|SwitchonENUM_StatusDrone (Variables|Default|GetStatusDrone)
    (:NewEnumerator0
      _)
    (:NewEnumerator2
      _))
  (if (< (Input|AxisValues|GetLeftThumbstrickY) 0.0)
    (if (<= (Variables|Default|GetHeight) 5e+01)
      (Variables|Default|SetZSpeed 5e+01)
      (Transformation|AddActorLocalOffset (Math|Vector|MakeVector 0.0 0.0 (Math|Interpolation|FInterpTo 0.0 (* (Variables|Default|GetZSpeed) (Input|AxisValues|GetLeftThumbstrickY)) (Utilities|Time|GetWorldDeltaSeconds) 1.0)) true false)
      (elif (<= (Variables|Default|GetHeight) 2.5e+02)
        (Variables|Default|SetZSpeed 1e+02)
        (Transformation|AddActorLocalOffset (Math|Vector|MakeVector 0.0 0.0 (Math|Interpolation|FInterpTo 0.0 (* (Variables|Default|GetZSpeed) (Input|AxisValues|GetLeftThumbstrickY)) (Utilities|Time|GetWorldDeltaSeconds) 1.0)) true false)
        (else
          (Variables|Default|SetZSpeed 3e+02)
          (Transformation|AddActorLocalOffset (Math|Vector|MakeVector 0.0 0.0 (Math|Interpolation|FInterpTo 0.0 (* (Variables|Default|GetZSpeed) (Input|AxisValues|GetLeftThumbstrickY)) (Utilities|Time|GetWorldDeltaSeconds) 1.0)) true false))))
    (else
      (Variables|Default|SetZSpeed 5e+02)
      (Transformation|AddActorLocalOffset (Math|Vector|MakeVector 0.0 0.0 (Math|Interpolation|FInterpTo 0.0 (* (Variables|Default|GetZSpeed) AxisValue) (Utilities|Time|GetWorldDeltaSeconds) 1.0)) true false))))

(event Input|AxisEvents|InputAxisRightThumbstrickY
  (params (AxisValue :type Float%20%28single-precision%29))
  ;[1 1 1] XYMove
  (switch Utilities|FlowControl|Switch|SwitchonENUM_StatusDrone (Variables|Default|GetStatusDrone)
    (:NewEnumerator0
      (bind _result (Math|Float|NegateFloat AxisValue)
        (:%20%20
          (Pawn|Input|AddMovementInput (Math|Vector|GetForwardVector (Variables|Default|GetBox_Chassis)) _result false))))))

(event Input|GamepadEvents|GamepadSpecialRight
  (params (Key :type Key%20Structure :default "None"))
  (bind _returnvalue (Game|GetPlayerController 0))
  ;[1 1 1] Pause
  (:Pressed
    (if (not (Game|IsGamePaused))
      (bind _returnvalue_2 (UserInterface|CreateWidget "/Game/RDSim/Blueprint/UI/Pause_Widget.Pause_Widget_C" _returnvalue))
      (UserInterface|Viewport|AddtoViewport _returnvalue_2 0)
      (Utilities|FlowControl|Delay 0.01)
      (Input|SetInputModeUIOnly _returnvalue _returnvalue_2 "DoNotLock" false)
      (Game|SetGamePaused true))))

(event Input|GamepadEvents|GamepadFaceButtonRight
  (params (Key :type Key%20Structure :default "None"))
  ;[1 1 1] RestartLevel
  (:Pressed
    (bind _returnvalue (Game|GetCurrentLevelName true))
    (Game|OpenLevel(byName) (Utilities|String|StringToName _returnvalue))))

(fn ConstructionScript)