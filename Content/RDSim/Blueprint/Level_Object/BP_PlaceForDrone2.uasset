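; BP_PlaceForDrone2 is a level object that marks a target place for the drone pawn.
; Every tick it finds the BP_DronePawn and shows the NSArrow effect only while the current mission is MS-6, deactivating it otherwise.
; When the drone pawn overlaps its Box, it calls Results on the drone HUD, regardless of the current mission.
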(event OnComponentBeginOverlap(Box)
  (params (OverlappedComponent :type Primitive%20Component%20Object%20Reference) (OtherActor :type Actor%20Object%20Reference) (OtherComp :type Primitive%20Component%20Object%20Reference) (OtherBodyIndex :type Integer) (bFromSweep :type Boolean) (SweepResult :type Hit%20Result%20Structure%20%28by%20ref%29))
  (bind _asbp_drone_pawn (Utilities|Casting|CastToBP_DronePawn OtherActor))
  (if true
    (Default|Results (Variables|/Game/RDSim/Blueprint/Prototype/DronFloating/BP_DronePawn.BP_DronePawn_C|GetDroneHUD _asbp_drone_pawn))))

(event EventTick
  (params (DeltaSeconds :type Float%20%28single-precision%29))
  (bind _ns_arrow (Variables|Default|GetNS_Arrow))
  (bind _returnvalue (Actor|GetActorOfClass "/Game/RDSim/Blueprint/Prototype/DronFloating/BP_DronePawn.BP_DronePawn_C"))
  (if (== (.name (Variables|/Game/RDSim/Blueprint/Prototype/DronFloating/QuestSystem/BP_Mission.BP_Mission_C|GetInfo (Variables|/Game/RDSim/Blueprint/Prototype/DronFloating/QuestSystem/BP_MissionManager.BP_MissionManager_C|GetCurrentMission (Variables|/Game/RDSim/Blueprint/Prototype/DronFloating/BP_DronePawn.BP_DronePawn_C|GetMissionManager _returnvalue)))) "MS-6")
    (Components|Activation|Activate _ns_arrow false)
    (else
      (Components|Activation|Deactivate _ns_arrow))))

(fn ConstructionScript)