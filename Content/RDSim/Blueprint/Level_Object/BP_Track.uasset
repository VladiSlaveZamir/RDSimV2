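; BP_Track is a spline-based track that lays out a numbered sequence of rings to be cleared in order.
; On BeginPlay it spawns a BP_Ring at each spline point, giving it a 1-based sequence number and a reference to the track.
; RingOver advances CurrentRingNum only for the matching number, then calls RingCompl on CurrentRing.
; CurrentRing is assigned only in the spawn loop, so it references the last ring spawned.
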(event Custom|RingOver
  (params (RingNum :type Integer))
  (bind _currentringnum (Variables|Default|GetCurrentRingNum))
  (if (== RingNum _currentringnum)
    (Math|Integer|IncrementInt _currentringnum
      (:%20%20
        (Default|RingCompl (Variables|Default|GetCurrentRing))))))

(event EventBeginPlay
  (bind _spline (Variables|Default|GetSpline))
  (for _index (range 0 (- (Spline|GetNumberOfSplinePoints _spline) 1))
    (bind _returnvalue (Game|SpawnActorfromClass "/Game/RDSim/Blueprint/Level_Object/BP_Ring.BP_Ring_C" (Spline|GetTransformatSplinePoint _spline _index "World" false) "Undefined" "MultiplyWithRoot" 0 0))
    (Variables|/Game/RDSim/Blueprint/Level_Object/BP_Ring.BP_Ring_C|SetSequenseNum _returnvalue (+ _index 1))
    (Variables|/Game/RDSim/Blueprint/Level_Object/BP_Ring.BP_Ring_C|SetSplineTrack _returnvalue self)
    (Variables|Default|SetCurrentRing _returnvalue)))

(event EventTick
  (params (DeltaSeconds :type Float%20%28single-precision%29)))

(fn ConstructionScript)