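; BP_Track2 is a spline-based track that lays out a course of rings to be completed in sequence.
; On BeginPlay it spawns a BP_Ring2 at each spline point's world transform, giving each a one-based sequence number and a reference back to the track.
; RingOver completes a ring and advances the counter only when its number matches the current one.
; The StartSpawnRings event is empty.
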(event Custom|StartSpawnRings)

(event Custom|RingOver
  (params (RingNum :type Integer) (CurrentRing :type BP%20Ring%202%20Object%20Reference))
  (bind _current_ring_num (Variables|Default|GetCurrent%20Ring%20Num))
  (if (== RingNum _current_ring_num)
    (Math|Integer|IncrementInt _current_ring_num
      (:%20%20
        (Default|RingCompl CurrentRing)))))

(event EventBeginPlay
  (bind _spline (Variables|Default|GetSpline))
  (for _index (range 0 (- (Spline|GetNumberOfSplinePoints _spline) 1))
    (bind _returnvalue (Game|SpawnActorfromClass "/Game/RDSim/Blueprint/Level_Object/BP_Ring2.BP_Ring2_C" (Spline|GetTransformatSplinePoint _spline _index "World" false) "Undefined" "MultiplyWithRoot" 0 0))
    (Variables|/Game/RDSim/Blueprint/Level_Object/BP_Ring2.BP_Ring2_C|SetSequense%20Num _returnvalue (+ _index 1))
    (Variables|/Game/RDSim/Blueprint/Level_Object/BP_Ring2.BP_Ring2_C|SetSpline%20Track _returnvalue self)))

(fn ConstructionScript)