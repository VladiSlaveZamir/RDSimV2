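; BP_Ring is a checkpoint ring on a drone race track that detects when the player's drone flies through it.
; A box overlap by a BP_DronePawn, while the ring is uncrossed, stores the pawn and reports the ring's sequence number to the SplineTrack via RingOver.
; RingCompl marks the ring crossed, updates the drone HUD's ring count and swaps the mesh to a completed material.
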(event OnComponentBeginOverlap(Box)
  (params (OverlappedComponent :type Primitive%20Component%20Object%20Reference) (OtherActor :type Actor%20Object%20Reference) (OtherComp :type Primitive%20Component%20Object%20Reference) (OtherBodyIndex :type Integer) (bFromSweep :type Boolean) (SweepResult :type Hit%20Result%20Structure%20%28by%20ref%29))
  (if (not (Variables|Default|GetIsCrossed))
    (bind _asbp_drone_pawn (Utilities|Casting|CastToBP_DronePawn OtherActor))
    (Variables|Default|SetAs%20BP%20Drone%20Pawn _asbp_drone_pawn)
    (Default|RingOver (Variables|Default|GetSplineTrack) (Variables|Default|GetSequenseNum) self)))

(event Custom|RingCompl
  (Variables|Default|SetIsCrossed true)
  (Default|InteractionCountRingEvent (Variables|/Game/RDSim/Blueprint/Prototype/DronFloating/BP_DronePawn.BP_DronePawn_C|GetDroneHUD (Variables|Default|GetAs%20BP%20Drone%20Pawn)))
  (Rendering|Material|SetMaterial (Variables|Default|GetStaticMesh) 0 "/Game/RDSim/Materials/M_CompleteRing.M_CompleteRing"))

(event EventBeginPlay)

(fn ConstructionScript)